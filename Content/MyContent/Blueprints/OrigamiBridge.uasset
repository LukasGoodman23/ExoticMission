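; Origami bridge actor that unfolds itself when play begins.
; An Unfold timeline, rate-scaled by UnfoldTime, drives every motion through lerps from a single track.
; It rolls the base mesh up and swings two groups of child meshes from folded to flat, with the second group yawed to face the opposite way.
; Two side cubes slide and stretch along Y in step with the unfolding.
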(event `self.ReceiveBeginPlay`
  (bind _unfold (`self.Unfold`))
  (set `self.RotationGroup1` (`|MakeArray` (`self.StaticMesh1`)))
  (set `self.RotationGroup2` (`|MakeArray` (`self.StaticMesh2`) (`self.StaticMesh3`) (`self.StaticMesh4`) (`self.StaticMesh5`)))
  (`TimelineComponent.SetPlayRate` _unfold (/ 1.0 (`self.UnfoldTime`)))
  (`TimelineComponent.PlayFromStart` _unfold))

(fn `UserConstructionScript`)